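; Main player character Blueprint: camera-relative movement, pitch-clamped camera, sword combat, damage and death.
; BeginPlay builds the HUD with player stats and a hidden boss bar, plus a pause menu that switches input modes.
; Combat mode reattaches the sword between back and hand, gating random attack montages and movement-locking blocks.
; A weapon capsule deals DoOnce-limited damage, reset after each attack; BPCLifeSystem tracks health and stamina, with blocks negating damage for stamina.
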(event OnComponentBeginOverlap(WeaponCapsule)
  (params (OverlappedComponent :type Primitive%20Component%20Object%20Reference) (OtherActor :type Actor%20Object%20Reference) (OtherComp :type Primitive%20Component%20Object%20Reference) (OtherBodyIndex :type Integer) (bFromSweep :type Boolean) (SweepResult :type Hit%20Result%20Structure%20%28by%20ref%29))
  ;[0.15 0.15 0.15 0.5] Applying damage to sword (using collision capsule)
  (Utilities|FlowControl|DoOnce false
    (:Completed
      (Game|Damage|ApplyDamage OtherActor 25.0 0 self))))

(event Custom|Refresh%20Damage
  ;[0.15 0.15 0.15 0.5] Applying damage to sword (using collision capsule)
  (Utilities|FlowControl|DoOnce false) ; enters at Reset
)

(event Custom|Unpause
  ;[0.15 0.15 0.15 0.5] Pause and Unpause logic
  (CallFunction|UnpauseSettings))

(event EventBeginPlay
  (bind _returnvalue (Game|GetPlayerController 0))
  ;[0.15 0.15 0.15 0.5] Invoking player HUD on screen (Main HUD and child "PlayerStats" HUD) + andjust postion and size on screen. And invoking Pause menu. And Boss HealthBar
  (bind _returnvalue_2 (UserInterface|CreateWidget "/Game/VGAProject/Interface/WB_PlayerHUD.WB_PlayerHUD_C" _returnvalue))
  (bind _output_get (Variables|Default|SetWB_PlayerHUD _returnvalue_2))
  (UserInterface|Viewport|AddtoViewport _output_get 0)
  (bind _returnvalue_3 (UserInterface|CreateWidget "/Game/VGAProject/Interface/WB_Player_Stats.WB_Player_Stats_C" _returnvalue))
  (bind _returnvalue_4 (Class|CanvasPanel|AddChildtoCanvas (Variables|/Game/VGAProject/Interface/WB_PlayerHUD.WB_PlayerHUD_C|GetPlayerHUD _output_get) _returnvalue_3))
  (Class|CanvasPanelSlot|SetPosition _returnvalue_4)
  (Class|CanvasPanelSlot|SetAutoSize _returnvalue_4 true)
  (bind _returnvalue_5 (UserInterface|CreateWidget "/Game/VGAProject/Interface/WB_Pause.WB_Pause_C" _returnvalue))
  (Variables|Default|SetWB_Pause _returnvalue_5)
  (bind _returnvalue_6 (UserInterface|CreateWidget "/Game/VGAProject/Interface/WB_Boss.WB_Boss_C" _returnvalue))
  (bind _output_get_2 (Variables|Default|SetWB_Boss _returnvalue_6))
  (bind _returnvalue_7 (Class|CanvasPanel|AddChildtoCanvas (Variables|/Game/VGAProject/Interface/WB_PlayerHUD.WB_PlayerHUD_C|GetPlayerHUD (Variables|Default|GetWB_PlayerHUD)) _output_get_2))
  (Class|CanvasPanelSlot|SetPosition _returnvalue_7 (Math|Vector2D|MakeVector2D 235.0 8.6e+02))
  (Class|CanvasPanelSlot|SetAutoSize _returnvalue_7 true)
  (Widget|SetVisibility _output_get_2 "Hidden") ; hide health bar before fight start
)

(event Collision|EventActorBeginOverlap
  (params (OtherActor :type Actor%20Object%20Reference)))

(event EventTick
  (params (DeltaSeconds :type Float%20%28single-precision%29))
  ;[0.15 0.15 0.15 0.5] Setting camera limitations on Pitch, so we can't get the camera deep into the model
  (CallFunction|CameraAngleSettings))

(event Input|ActionEvents|InputActionPause
  (params (Key :type Key%20Structure :default "None"))
  ;[0.15 0.15 0.15 0.5] Pause and Unpause logic
  (:Pressed
    (CallFunction|PauseSettings)))

(event Input|AxisEvents|InputAxisLookUp
  (params (AxisValue :type Float%20%28single-precision%29))
  ;[0.15 0.15 0.15 0.5] Adding an option for looking up and down
  (Pawn|Input|AddControllerPitchInput AxisValue))

(event Input|AxisEvents|InputAxisLookRight
  (params (AxisValue :type Float%20%28single-precision%29))
  ;[0.15 0.15 0.15 0.5] Adding an option for looking right and left
  (Pawn|Input|AddControllerYawInput AxisValue))

(event Input|AxisEvents|InputAxisMoveForwardBack
  (params (AxisValue :type Float%20%28single-precision%29))
  ;[0.15 0.15 0.15 0.5] Adding an option to control a character from the keyboard. We can't move while holding block
  (if (not (and (Variables|Default|GetCombatMode) (Variables|Default|GetBlocking)))
    (Pawn|Input|AddMovementInput (Math|Vector|GetForwardVector (Math|Rotator|MakeRotator 0.0 0.0 (.yaw (Pawn|GetControlRotation :!class /Script/Engine.Pawn)))) AxisValue false)))

(event Input|AxisEvents|InputAxisMoveRightLeft
  (params (AxisValue :type Float%20%28single-precision%29))
  ;[0.15 0.15 0.15 0.5] Adding an option to control a character from the keyboard. We can't move while holding block
  (if (not (and (Variables|Default|GetCombatMode) (Variables|Default|GetBlocking)))
    (Pawn|Input|AddMovementInput (Math|Vector|GetRightVector (Math|Rotator|MakeRotator 0.0 0.0 (.yaw (Pawn|GetControlRotation :!class /Script/Engine.Pawn)))) AxisValue false)))

(fn ConstructionScript)

(fn ReduceDamage
  (params (IncomingDamage :type Float%20%28double-precision%29))
  (bind _bpc_life_system (Variables|Default|GetBPC_Life_System))
  ;[0.15 0.15 0.15 0.5] 2 conditions. If blocking, doesn't getting damage. If not, getting full incoming damage + checking if we have enough stamina for blocking
  (if (Variables|Default|GetBlocking)
    (Audio|PlaySoundatLocation "/Game/VGAProject/Sound/CombatCue/SC_Blocked.SC_Blocked" "0, 0, 0" "0, 0, 0" 1.0 1.0 0.0 0 0 0 0) ; Block sound
    (Default|StaminaChange _bpc_life_system 10)
    (if (== (Variables|/Game/VGAProject/Characters/Main_Character/Blueprint/BPC_Life_System.BPC_Life_System_C|GetCurrentStamina _bpc_life_system) 0)
      (Variables|Default|SetBlocking false))
    (return 0)
    (else
      (Audio|PlaySoundatLocation "/Game/VGAProject/Sound/CombatCue/SC_WeaponHit.SC_WeaponHit" "0, 0, 0" "0, 0, 0" 1.0 1.0 0.0 0 0 0 0) ; Hit Sound
      (Audio|PlaySoundatLocation "/Game/VGAProject/Sound/VoiceCue/SC_VoiceHit.SC_VoiceHit" "0, 0, 0" "0, 0, 0" 1.0 1.0 0.0 0 0 0 0) ; Voice Hit Sound
      (return (Math|Float|Truncate IncomingDamage)))))

(fn SetCollisionOff
  (Collision|SetCollisionEnabled (Variables|Character|GetMesh) "NoCollision")
  (Collision|SetCollisionEnabled (Variables|Default|GetWeaponCapsule) "NoCollision")
  (Collision|SetCollisionEnabled (Variables|Collision|GetCapsuleComponent) "NoCollision"))

(fn CameraAngleSettings
  (bind _returnvalue (Pawn|GetControlRotation :!class /Script/Engine.Pawn))
  (Pawn|SetControlRotation (Game|GetPlayerController 0) (Math|Rotator|MakeRotator (.roll _returnvalue) (Math|Float|ClampAngle (.pitch _returnvalue) -45.0 45.0) (.yaw _returnvalue)))
  (return))

(fn PauseSettings
  (bind _returnvalue (Game|GetPlayerController 0))
  (bind (_sizex _sizey) (HUD|GetViewportSize _returnvalue))
  ;[0.15 0.15 0.15 0.5] Logic of Pause Menu. Frozen game state and showing pause widget in a main canvas. Protection from invoking multiple pause widget. Getting Size of viewport, adjusting menu in the middle of the screen. Turning on mouse cursor and turning off in-game control buttons (attack, block)
  (Utilities|IsValid (Variables|Default|GetWB_PlayerHUD) ; check if exist
    (:Is%20Valid
      (Utilities|IsValid (Variables|Default|GetWB_Pause) ; check if exist
        (:Is%20Valid
          (if (not (Variables|Default|GetGamePaused)) ; If true (game in pause) we do nothing
            (Utilities|FlowControl|DoOnce false :!label _label ; secure from spamming
              (:Completed
                (Game|SetGamePaused true) ; pausing game state
                (bind _returnvalue_2 (Class|CanvasPanel|AddChildtoCanvas (Variables|/Game/VGAProject/Interface/WB_PlayerHUD.WB_PlayerHUD_C|GetPlayerHUD (Variables|Default|GetWB_PlayerHUD)) (Variables|Default|GetWB_Pause))) ; adding on main HUD pause widget
                (Class|CanvasPanelSlot|SetPosition _returnvalue_2 (Math|Vector2D|MakeVector2D (- (Math|Conversions|ToFloat(Integer) (/ _sizex 2)) 275.0) (- (Math|Conversions|ToFloat(Integer) (/ _sizey 2)) 275.0))) ; position of pause widget on screne
                (Class|CanvasPanelSlot|SetAutoSize _returnvalue_2 true)
                (Variables|/Script/Engine.PlayerController|SetbShowMouseCursor _returnvalue true) ; showing mouse cursor in the pause widget
                (Input|SetInputModeUIOnly _returnvalue (Variables|Default|GetWB_Pause) "LockOnCapture" false) ; turn off all in-game control buttons, while in pause widget
                (Variables|Default|SetGamePaused true) ; secure from invoking pause widget, while we already in pause menu
                (goto _label Reset)))))))))

(fn UnpauseSettings
  (bind _returnvalue (Game|GetPlayerController 0))
  ;[0.15 0.15 0.15 0.5] Logic of Unpause Menu. Unfrozen game state and disable pause widget from the main canvas. Protection from multiple spamming resume button.Turning off mouse cursor and turning on in-game control buttons (attack, block)
  (Utilities|IsValid (Variables|Default|GetWB_PlayerHUD) ; check if exist
    (:Is%20Valid
      (Utilities|IsValid (Variables|Default|GetWB_Pause) ; check if exist
        (:Is%20Valid
          (if (Variables|Default|GetGamePaused) ; If true (game in pause) we do nothing
            (Utilities|FlowControl|DoOnce false :!label _label ; secure from spamming
              (:Completed
                (Variables|Default|SetGamePaused false) ; when pause menu close
                (Input|SetInputModeGameOnly _returnvalue false) ; turn on all in-game control buttons again
                (Variables|/Script/Engine.PlayerController|SetbShowMouseCursor _returnvalue false) ; disable mouse cursor
                (Widget|RemovefromParent (Variables|Default|GetWB_Pause)) ; disable pause widget from main HUD
                (Game|SetGamePaused false) ; unfrozen game state
                (goto _label Reset)))))))))

(event Game|Damage|EventAnyDamage
  (params (Damage :type Float%20%28single-precision%29) (DamageType :type Damage%20Type%20Object%20Reference) (InstigatedBy :type Controller%20Object%20Reference) (DamageCauser :type Actor%20Object%20Reference))
  (bind _returnvalue (Game|GetPlayerController 0))
  (bind _bpc_life_system (Variables|Default|GetBPC_Life_System))
  ;[0.15 0.15 0.15 0.5] Logic of getting damage and destroing main character with animation + function of blocking damage. Control enabling/disabling
  (bind _outputdamage (CallFunction|ReduceDamage Damage))
  (Default|HealthChange _bpc_life_system (Math|Conversions|ToFloat(Integer) _outputdamage))
  (if (== (Variables|/Game/VGAProject/Characters/Main_Character/Blueprint/BPC_Life_System.BPC_Life_System_C|GetCurrentHealth _bpc_life_system) 0)
    (Variables|Default|SetDead true) ; variable for enemy to know player is dead
    (CallFunction|SetCollisionOff) ; turn off all collision, so player can't get damage
    (Audio|PlaySoundatLocation "/Game/VGAProject/Sound/VoiceCue/SC_VoiceDeath.SC_VoiceDeath" "0, 0, 0" "0, 0, 0" 1.0 1.0 0.0 0 0 0 0) ; death sound
    (Input|DisableInput _returnvalue) ; when dead you can't control character
    (bind _returnvalue_2 (Animation|PlayAnimMontage "/Game/VGAProject/Characters/Main_Character/Animation/Death/AM_Death.AM_Death" 1.0 "None"))
    (Utilities|FlowControl|Delay _returnvalue_2) ; delay until animation ends
    (Utilities|FlowControl|Delay 2.0) ; 2 seconds on a ground more
    (Actor|DestroyActor)
    (Input|EnableInput _returnvalue) ; turn on contorlling after death animation
  ))

(event Input|ActionEvents|InputActionCombatMode
  (params (Key :type Key%20Structure :default "None"))
  (bind _sword (Variables|Default|GetSword))
  ;[0.15 0.15 0.15 0.5] Switching between modes by X key + enabling the animation of drawing a sword + disabling blocking if we switching to non-combat mode
  (:Pressed
    (if (not (Variables|Default|GetAttacking))
      (Utilities|FlowControl|DoOnce false :!label _label
        (:Completed
          (Utilities|FlowControl|FlipFlop
            (:A
              (Animation|PlayAnimMontage "/Game/VGAProject/Characters/Main_Character/Animation/Locomotion/Combat/AM_Sheath.AM_Sheath" 1.0 "None")
              (Utilities|FlowControl|Delay 0.96)
              (Audio|PlaySoundatLocation "/Game/VGAProject/Sound/CombatCue/SC_WeaponOn.SC_WeaponOn" "0, 0, 0" "0, 0, 0" 1.0 1.0 0.0 0 0 0 0) ; Weapon Sheath On sound
              (Transformation|AttachComponentToComponent _sword (Variables|Default|GetWeaponOn) "None" "SnapToTarget" "SnapToTarget" "KeepRelative" true) ; we attaching sword to arm
              (Utilities|FlowControl|Delay 0.71)
              (Variables|Default|SetCombatMode true)
              (goto _label Reset))
            (:B
              (Animation|PlayAnimMontage "/Game/VGAProject/Characters/Main_Character/Animation/Locomotion/Combat/AM_Sheath.AM_Sheath" 1.0 "None")
              (Utilities|FlowControl|Delay 0.96)
              (Audio|PlaySoundatLocation "/Game/VGAProject/Sound/CombatCue/SC_WeaponOff.SC_WeaponOff" "0, 0, 0" "0, 0, 0" 1.0 1.0 0.0 0 0 0 0) ; Weapon Sheath Off sound
              (Transformation|AttachComponentToComponent _sword (Variables|Default|GetWeaponOff) "None" "SnapToTarget" "SnapToTarget" "KeepRelative" true) ; we attaching sword to back
              (Utilities|FlowControl|Delay 0.71)
              (Variables|Default|SetCombatMode false)
              (Variables|Default|SetBlocking false)
              (goto _label Reset))))))))

(event Input|ActionEvents|InputActionAttack
  (params (Key :type Key%20Structure :default "None"))
  ;[0.15 0.15 0.15 0.5] Attacking logic. Using random 50/50 to play 2 independent and different attack animations (plus security from attacking from non-combat mode)
  (:Pressed
    (if (and (Variables|Default|GetCombatMode) (not (Variables|Default|GetBlocking))) ; Allow to attack only in combat mode
      (Utilities|FlowControl|DoOnce false :!label _label
        (:Completed
          (Variables|Default|SetAttacking true) ; securtiy from multiple attacks during one animation playtime
          (bind _returnvalue (Animation|PlayAnimMontage (select (Math|Random|RandomBool) "/Game/VGAProject/Characters/Main_Character/Animation/Combat/AM_Attack2.AM_Attack2" "/Game/VGAProject/Characters/Main_Character/Animation/Combat/AM_Attack1.AM_Attack1") 1.0 "None"))
          (Utilities|FlowControl|Delay _returnvalue)
          (Variables|Default|SetAttacking false)
          (CallFunction|RefreshDamage) ; Aplly damage for each attack
          (goto _label Reset))))))

(event Input|ActionEvents|InputActionBlocking
  (params (Key :type Key%20Structure :default "None"))
  (bind _bpc_life_system (Variables|Default|GetBPC_Life_System))
  (bind _combatmode (Variables|Default|GetCombatMode))
  (bind _attacking (Variables|Default|GetAttacking))
  (bind _returnvalue (not _attacking))
  (bind _currentstamina (Variables|/Game/VGAProject/Characters/Main_Character/Blueprint/BPC_Life_System.BPC_Life_System_C|GetCurrentStamina _bpc_life_system))
  (bind _returnvalue_2 (>= _currentstamina 10))
  (bind _returnvalue_3 (Math|Boolean|ANDBoolean _combatmode _returnvalue _returnvalue_2))
  ;[0.15 0.15 0.15 0.5] Visual part of blocking. If pressing RMB and holding we blocking, if releasing button block ends. Plus security for blocking in combat mode only and current stamina check
  (:Pressed
    (if _returnvalue_3
      (Variables|Default|SetBlocking true)))
  (:Released
    (if _returnvalue_3
      (Variables|Default|SetBlocking false))))