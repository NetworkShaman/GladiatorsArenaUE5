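; Life system component in the main character's folder that tracks integer health and stamina, both set to their maximums on BeginPlay.
; HealthChange and StaminaChange subtract incoming damage or spent stamina with a floor of zero, truncating damage to an integer.
; Tick runs through a Delay to regenerate stamina about once per second, capped at the maximum.
; HealthRecovery offers similar capped healing but is not called within this component.
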(event EventBeginPlay
  ;[0.15 0.15 0.15 0.5] Setting Max Health/Stamina, Current Health/Stamina
  (Variables|Default|SetCurrentHealth (Variables|Default|GetMaxHealth))
  (Variables|Default|SetCurrentStamina (Variables|Default|GetMaxStamina)))

(event EventTick
  (params (DeltaSeconds :type Float%20%28single-precision%29))
  ;[0.15 0.15 0.15 0.5] Stamina regeneration every single second
  (Utilities|FlowControl|Delay 1.0)
  (CallFunction|StaminaRecovery))

(fn HealthChange
  (params (IncomingDamage :type Float%20%28double-precision%29))
  (Variables|Default|SetCurrentHealth (Math|Integer|SelectInt (- (Variables|Default|GetCurrentHealth) (Math|Float|Truncate IncomingDamage)) 0 (> (- (Variables|Default|GetCurrentHealth) (Math|Float|Truncate IncomingDamage)) 0))))

(fn StaminaChange
  (params (StaminaSpent :type Integer))
  (Variables|Default|SetCurrentStamina (Math|Integer|SelectInt (- (Variables|Default|GetCurrentStamina) StaminaSpent) 0 (> (- (Variables|Default|GetCurrentStamina) StaminaSpent) 0))))

(fn StaminaRecovery
  (bind _maxstamina (Variables|Default|GetMaxStamina))
  (Variables|Default|SetCurrentStamina (Math|Integer|SelectInt (+ (Variables|Default|GetCurrentStamina) 2) _maxstamina (< (+ (Variables|Default|GetCurrentStamina) 2) _maxstamina))))

(fn HealthRecovery
  (bind _maxhealth (Variables|Default|GetMaxHealth))
  (Variables|Default|SetCurrentHealth (Math|Integer|SelectInt (+ (Variables|Default|GetCurrentHealth) 1) _maxhealth (< (+ (Variables|Default|GetCurrentHealth) 1) _maxhealth))))