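; Boss enemy character with a large health pool that drives the boss health bar on the player's widget through a delayed Tick.
; Attack plays a light or randomly chosen heavy montage, flagging HeavyAttack during the latter.
; Hand collision overlaps damage only the player, with per-hand DoOnce gates re-armed by RefreshDamage.
; Incoming damage feeds BPCLifeSystem; zero health disables collision, plays death sound and montage, then destroys the actor.
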(event OnComponentBeginOverlap(LeftHand)
  (params (OverlappedComponent :type Primitive%20Component%20Object%20Reference) (OtherActor :type Actor%20Object%20Reference) (OtherComp :type Primitive%20Component%20Object%20Reference) (OtherBodyIndex :type Integer) (bFromSweep :type Boolean) (SweepResult :type Hit%20Result%20Structure%20%28by%20ref%29))
  ;[0.15 0.15 0.15 0.5] Using Collision Capsule applying on boss hands we can deal damage using "Apply Damage" function. Plus logic of ignoring damage from enemy to another enemies, so they can deal damage to player only. And special heavy attack
  (if (== OtherActor (Variables|Default|GetRefPlayer))
    (Utilities|FlowControl|DoOnce false
      (:Completed
        (Game|Damage|ApplyDamage OtherActor 4e+01 0 0)))))

(event OnComponentBeginOverlap(RightHand)
  (params (OverlappedComponent :type Primitive%20Component%20Object%20Reference) (OtherActor :type Actor%20Object%20Reference) (OtherComp :type Primitive%20Component%20Object%20Reference) (OtherBodyIndex :type Integer) (bFromSweep :type Boolean) (SweepResult :type Hit%20Result%20Structure%20%28by%20ref%29))
  ;[0.15 0.15 0.15 0.5] Using Collision Capsule applying on boss hands we can deal damage using "Apply Damage" function. Plus logic of ignoring damage from enemy to another enemies, so they can deal damage to player only. And special heavy attack
  (if (== OtherActor (Variables|Default|GetRefPlayer))
    (Utilities|FlowControl|DoOnce false
      (:Completed
        (Game|Damage|ApplyDamage OtherActor 2e+01 0 0)))))

(event Custom|Attack
  ;[0.15 0.15 0.15 0.5] Logic of boss attack. He is a unique enemy with 2 attacks that deal different damage. Heavy attack procs with 20 % chance
  (Utilities|FlowControl|DoOnce false :!label _label
    (:Completed
      (if (Math|Random|RandomBoolwithWeight 0.2)
        (Variables|Default|SetHeavyAttack true)
        (bind _returnvalue (Animation|PlayAnimMontage "/Game/VGAProject/Characters/Enemies/BossEnemy/Animation/Combat/AM_BossHeavyAttack.AM_BossHeavyAttack" 1.0 "None")) ; Boss heavy attack
        (Utilities|FlowControl|Delay (/ _returnvalue 1.1))
        (Variables|Default|SetHeavyAttack false)
        (goto _label Reset)
        (else
          (bind _returnvalue_2 (Animation|PlayAnimMontage "/Game/VGAProject/Characters/Enemies/BossEnemy/Animation/Combat/AM_BossLightAttack.AM_BossLightAttack" 1.0 "None")) ; Boss light standart attack
          (Utilities|FlowControl|Delay (/ _returnvalue_2 1.1))
          (goto _label Reset))))))

(event Custom|RefreshDamage
  ;[0.15 0.15 0.15 0.5] Using Collision Capsule applying on boss hands we can deal damage using "Apply Damage" function. Plus logic of ignoring damage from enemy to another enemies, so they can deal damage to player only. And special heavy attack
  (Utilities|FlowControl|Sequence
    (:then_0
      (Utilities|FlowControl|DoOnce false) ; enters at Reset
    )
    (:then_1
      (Utilities|FlowControl|DoOnce false) ; enters at Reset
    )))

(event EventBeginPlay
  (bind _bpc_life_system (Variables|Default|GetBPC_Life_System))
  ;[0.15 0.15 0.15 0.5] Getting reference on a player and setting boss max health
  (bind _asbp_ch_player (Utilities|Casting|CastToBP_CH_Player (Game|GetPlayerCharacter 0)))
  (Variables|Default|SetRefPlayer _asbp_ch_player)
  (bind _output_get (Variables|/Game/VGAProject/Characters/Main_Character/Blueprint/BPC_Life_System.BPC_Life_System_C|SetMaxHealth _bpc_life_system 500))
  (Variables|/Game/VGAProject/Characters/Main_Character/Blueprint/BPC_Life_System.BPC_Life_System_C|SetCurrentHealth _bpc_life_system _output_get))

(event Game|Damage|EventAnyDamage
  (params (Damage :type Float%20%28single-precision%29) (DamageType :type Damage%20Type%20Object%20Reference) (InstigatedBy :type Controller%20Object%20Reference) (DamageCauser :type Actor%20Object%20Reference))
  (bind _bpc_life_system (Variables|Default|GetBPC_Life_System))
  ;[0.15 0.15 0.15 0.5] Logic of taking damage by boss and his destruction with animation and disabling collision
  (Audio|PlaySoundatLocation "/Game/VGAProject/Sound/CombatCue/SC_WeaponHit.SC_WeaponHit" "0, 0, 0" "0, 0, 0" 1.0 1.0 0.0 0 0 0 0) ; hit
  (Audio|PlaySoundatLocation "/Game/VGAProject/Sound/VoiceCue/SC_VoiceBossHit.SC_VoiceBossHit" "0, 0, 0" "0, 0, 0" 1.0 1.0 0.0 0 0 0 0) ; voice hit
  (Default|HealthChange _bpc_life_system Damage)
  (if (== (Variables|/Game/VGAProject/Characters/Main_Character/Blueprint/BPC_Life_System.BPC_Life_System_C|GetCurrentHealth _bpc_life_system) 0)
    (Variables|Default|SetDead true)
    (CallFunction|SetCollisionOff)
    (Audio|PlaySoundatLocation "/Game/VGAProject/Sound/VoiceCue/SC_VoiceBossDeath.SC_VoiceBossDeath" "0, 0, 0" "0, 0, 0" 1.0 1.0 0.0 0 0 0 0) ; boss death sound
    (bind _returnvalue (Animation|PlayAnimMontage "/Game/VGAProject/Characters/Enemies/BossEnemy/Animation/Death/AM_BossDeath.AM_BossDeath" 1.0 "None"))
    (Utilities|FlowControl|Delay _returnvalue)
    (Actor|DestroyActor)))

(event EventTick
  (params (DeltaSeconds :type Float%20%28single-precision%29))
  (bind _bpc_life_system (Variables|Default|GetBPC_Life_System))
  (bind _refplayer (Variables|Default|GetRefPlayer))
  (bind _maxhealth (Variables|/Game/VGAProject/Characters/Main_Character/Blueprint/BPC_Life_System.BPC_Life_System_C|GetMaxHealth _bpc_life_system))
  (bind _returnvalue (Math|Conversions|ToFloat(Integer) _maxhealth))
  ;[0.15 0.15 0.15 0.5] Logic of Boss Health bar Widget. Because we have more then 100 hp we need to make a conversion to float for correct work. And stopping attack animation after boss dead
  (Utilities|FlowControl|Delay 0.2)
  (Utilities|IsValid _refplayer
    (:Is%20Valid
      (Progress|SetPercent (Variables|/Game/VGAProject/Interface/WB_Boss.WB_Boss_C|GetBossHealth (Variables|/Game/VGAProject/Characters/Main_Character/Blueprint/BP_CH_Player.BP_CH_Player_C|GetWB_Boss _refplayer)) (/ (Math|Float|Clamp(Float) (Math|Conversions|ToFloat(Integer) (Variables|/Game/VGAProject/Characters/Main_Character/Blueprint/BPC_Life_System.BPC_Life_System_C|GetCurrentHealth _bpc_life_system)) 0.0 _returnvalue) _returnvalue))
      (if (Variables|Default|GetDead)
        (Animation|StopAnimMontage "/Game/VGAProject/Characters/Enemies/BossEnemy/Animation/Combat/AM_BossLightAttack.AM_BossLightAttack")
        (Animation|StopAnimMontage "/Game/VGAProject/Characters/Enemies/BossEnemy/Animation/Combat/AM_BossHeavyAttack.AM_BossHeavyAttack")))))

(fn ConstructionScript)

(fn SetCollisionOff
  (Collision|SetCollisionEnabled (Variables|Default|GetRightHand) "NoCollision")
  (Collision|SetCollisionEnabled (Variables|Default|GetLeftHand) "NoCollision")
  (Collision|SetCollisionEnabled (Variables|Character|GetMesh) "NoCollision")
  (Collision|SetCollisionEnabled (Variables|Collision|GetCapsuleComponent) "NoCollision"))