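; Enemy character Blueprint that handles melee attacks, damage, death and victory celebration.
; Attack plays random montages behind a DoOnce-plus-delay gate, while the weapon capsule damages only the player, once until RefreshDamage resets it.
; AnyDamage feeds BPCLifeSystem, then at zero health plays death sound and montage and destroys the actor.
; Tick turns the health-bar widget toward the player's camera, shows it only nearby while alive, updates it and stops attack montages after death.
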(event OnComponentBeginOverlap(EnemyWeaponCapsule)
  (params (OverlappedComponent :type Primitive%20Component%20Object%20Reference) (OtherActor :type Actor%20Object%20Reference) (OtherComp :type Primitive%20Component%20Object%20Reference) (OtherBodyIndex :type Integer) (bFromSweep :type Boolean) (SweepResult :type Hit%20Result%20Structure%20%28by%20ref%29))
  ;[0.15 0.15 0.15 0.5] Using Collision Capsule applying on enemy weapon we can deal damage using "Apply Damage" function. Plus logic of ignoring damage from enemy to another enemies, so they can deal damage to player only
  (bind _asbp_ch_player (Utilities|Casting|CastToBP_CH_Player (Game|GetPlayerCharacter 0)))
  (if (== _asbp_ch_player OtherActor)
    (Utilities|FlowControl|DoOnce false
      (:Completed
        (Game|Damage|ApplyDamage OtherActor 1e+01 0 self)))))

(event Custom|Attack
  ;[0.15 0.15 0.15 0.5] Logic of enemy attack. Enemy with little delay commiting one attack with different animations. "Do once" with delay is protection from spamming
  (Utilities|FlowControl|DoOnce false :!label _label
    (:Completed
      (bind _returnvalue (Animation|PlayAnimMontage (select (Math|Random|RandomBool) "/Game/VGAProject/Characters/Enemies/MorakEnemy/Animation/Combat/AM_EnemyAttack_2.AM_EnemyAttack_2" "/Game/VGAProject/Characters/Enemies/MorakEnemy/Animation/Combat/AM_EnemyAttack_1.AM_EnemyAttack_1") 1.0 "None"))
      (Utilities|FlowControl|Delay (+ _returnvalue 0.1))
      (goto _label Reset))))

(event Custom|RefreshDamage
  ;[0.15 0.15 0.15 0.5] Using Collision Capsule applying on enemy weapon we can deal damage using "Apply Damage" function. Plus logic of ignoring damage from enemy to another enemies, so they can deal damage to player only
  (Utilities|FlowControl|DoOnce false) ; enters at Reset
)

(event Custom|Triumph
  ;[0.15 0.15 0.15 0.5] If enemy kill main character he start to celebrate the victory using two animations
  (Utilities|FlowControl|DoOnce false
    (:Completed
      (Animation|PlayAnimMontage (select (Math|Random|RandomBool) "/Game/VGAProject/Characters/Enemies/MorakEnemy/Animation/Triumph/AM_EnemyTriumph2.AM_EnemyTriumph2" "/Game/VGAProject/Characters/Enemies/MorakEnemy/Animation/Triumph/AM_EnemyTriumph1.AM_EnemyTriumph1") 1.0 "None"))))

(event EventBeginPlay)

(event Collision|EventActorBeginOverlap
  (params (OtherActor :type Actor%20Object%20Reference)))

(event EventTick
  (params (DeltaSeconds :type Float%20%28single-precision%29))
  ;[0.15 0.15 0.15 0.5] Setting widget rotation. Setting enemy Health bar Widget. And stopping enemies attack animations after they dead
  (CallFunction|SetWidgetRotation)
  (CallFunction|SetEnemyHealthBar)
  (if (Variables|Default|GetDead)
    (Animation|StopAnimMontage "/Game/VGAProject/Characters/Enemies/MorakEnemy/Animation/Combat/AM_EnemyAttack_1.AM_EnemyAttack_1") ; stop animation 1
    (Animation|StopAnimMontage "/Game/VGAProject/Characters/Enemies/MorakEnemy/Animation/Combat/AM_EnemyAttack_2.AM_EnemyAttack_2") ; stop animation 2
  ))

(event Game|Damage|EventAnyDamage
  (params (Damage :type Float%20%28single-precision%29) (DamageType :type Damage%20Type%20Object%20Reference) (InstigatedBy :type Controller%20Object%20Reference) (DamageCauser :type Actor%20Object%20Reference))
  (bind _bpc_life_system (Variables|Default|GetBPC_Life_System))
  ;[0.15 0.15 0.15 0.5] Logic of getting damage and destroing enemy with animation and stopping every attack animation
  (Audio|PlaySoundatLocation "/Game/VGAProject/Sound/CombatCue/SC_WeaponHit.SC_WeaponHit" "0, 0, 0" "0, 0, 0" 1.0 1.0 0.0 0 0 0 0) ; Hit Sound
  (Audio|PlaySoundatLocation "/Game/VGAProject/Sound/VoiceCue/SC_VoiceHit.SC_VoiceHit" "0, 0, 0" "0, 0, 0" 1.0 1.0 0.0 0 0 0 0) ; Voice Hit Sound
  (Default|HealthChange _bpc_life_system Damage)
  (if (== (Variables|/Game/VGAProject/Characters/Main_Character/Blueprint/BPC_Life_System.BPC_Life_System_C|GetCurrentHealth _bpc_life_system) 0)
    (Variables|Default|SetDead true)
    (Audio|PlaySoundatLocation "/Game/VGAProject/Sound/VoiceCue/SC_VoiceEnemyDeath.SC_VoiceEnemyDeath" "0, 0, 0" "0, 0, 0" 1.0 1.0 0.0 0 0 0 0) ; enemy death sound
    (bind _returnvalue (Animation|PlayAnimMontage "/Game/VGAProject/Characters/Enemies/MorakEnemy/Animation/Death/AM_EnemyDeath.AM_EnemyDeath" 1.0 "None"))
    (Utilities|FlowControl|Delay _returnvalue) ; delay until animation ends
    (Utilities|FlowControl|Delay 2.0) ; 2 seconds on a ground more
    (Actor|DestroyActor)))

(fn ConstructionScript)

(fn SetWidgetRotation
  (bind _widget (Variables|Default|GetWidget))
  (bind _widget_2 (Variables|Default|GetWidget))
  ;[0.15 0.15 0.15 0.5] We invoke player's blueprint to get character's camera. Then getting position of player camera and enemy health bar, calculate new coordinates for rotation and showing to player's camera. If distance to enemy is more then 1000, we will not see health bar
  (bind _asbp_ch_player (Utilities|Casting|CastToBP_CH_Player (Game|GetPlayerCharacter 0)))
  (Transformation|SetWorldRotation _widget_2 (Math|Rotator|FindLookatRotation (Transformation|GetWorldLocation _widget_2) (Transformation|GetWorldLocation (Variables|/Game/VGAProject/Characters/Main_Character/Blueprint/BP_CH_Player.BP_CH_Player_C|GetCamera _asbp_ch_player))) false false) ; set rotation of health bar
  (if (and (< (Transformation|GetDistanceTo _asbp_ch_player self) 1e+03) (not (Variables|Default|GetDead)))
    (Rendering|SetVisibility _widget true false)
    (else
      (Rendering|SetVisibility _widget false false)))
  (return))

(fn SetCollisionOff
  (Collision|SetCollisionEnabled (Variables|Default|GetEnemyWeaponCapsule) "NoCollision")
  (Collision|SetCollisionEnabled (Variables|Collision|GetCapsuleComponent) "NoCollision")
  (Collision|SetCollisionEnabled (Variables|Character|GetMesh) "NoCollision"))

(fn SetEnemyHealthBar
  (bind _bpc_life_system (Variables|Default|GetBPC_Life_System))
  ;[0.15 0.15 0.15 0.5] Invoking BPC Life System with Current/Max Health. All data will be sent to Health bar variable to show in enemy Health widget
  (bind _aswb_enemy_stats (Utilities|Casting|CastToWB_Enemy_Stats (UserInterface|GetUserWidgetObject (Variables|Default|GetWidget))))
  (Progress|SetPercent (Variables|/Game/VGAProject/Interface/WB_Enemy_Stats.WB_Enemy_Stats_C|GetEnemyHeathBar _aswb_enemy_stats) (/ (Math|Conversions|ToFloat(Integer) (Math|Integer|Clamp(Integer) (Variables|/Game/VGAProject/Characters/Main_Character/Blueprint/BPC_Life_System.BPC_Life_System_C|GetCurrentHealth _bpc_life_system) 0 (Variables|/Game/VGAProject/Characters/Main_Character/Blueprint/BPC_Life_System.BPC_Life_System_C|GetMaxHealth _bpc_life_system))) 1e+02))
  (return))