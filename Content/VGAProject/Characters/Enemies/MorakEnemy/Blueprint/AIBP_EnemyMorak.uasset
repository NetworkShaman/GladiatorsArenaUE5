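; AI controller for the Morak enemy that chases and attacks the player, patrols when none is near, and celebrates once the player dies.
; BeginPlay caches both characters; Tick, throttled by a delay, calls FindEnemy, a distance check that also reports player death.
; DoOnce gates each AI MoveTo: reaching the player triggers Attack and another search, while patrol picks random reachable points around the enemy.
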(event EventBeginPlay
  ;[0.15 0.15 0.15 0.5] Invoking enemy character and invoking main character
  (Utilities|FlowControl|Delay 0.2) ; Delay on invoke
  (bind _asbp_ch_enemy (Utilities|Casting|CastToBP_CH_Enemy (Pawn|GetControlledPawn)))
  (Variables|Default|SetRefEnemy _asbp_ch_enemy)
  (bind _asbp_ch_player (Utilities|Casting|CastToBP_CH_Player (Game|GetPlayerCharacter 0)))
  (Variables|Default|SetRefPlayer _asbp_ch_player))

(event EventTick
  (params (DeltaSeconds :type Float%20%28single-precision%29))
  (bind _refenemy (Variables|Default|GetRefEnemy))
  ;[0.15 0.15 0.15 0.5] Logic of detecting and walking to player. With 0.5 seconds delay enemy try to find a character. If found then using "AI MoveTo" function Pawn (Enemy) move to Target (Player). If enemy can't find player, with a second delay he will try to detect character again. If enemy found and already move to player, he start to attack him
  (Utilities|IsValid _refenemy ; Checking if enemy is alive
    (:Is%20Valid
      (Utilities|IsValid (Variables|Default|GetRefPlayer) ; Checking if player is alive
        (:Is%20Valid
          (if (not (Variables|/Game/VGAProject/Characters/Enemies/MorakEnemy/Blueprint/BP_CH_Enemy.BP_CH_Enemy_C|GetDead _refenemy)) :!label _label
            (Utilities|FlowControl|Delay 0.5)
            (bind (_found _playerdead) (CallFunction|FindEnemy))
            (if _playerdead ; if player not dead run following code
              (Default|Triumph _refenemy) ; if branch was true, enemy celebrates victory
              (elif _found
                (Utilities|FlowControl|DoOnce false :!label _label_2
                  (:Completed
                    (AI|AIMoveTo (Variables|Default|GetRefEnemy) "0, 0, 0" (Variables|Default|GetRefPlayer) 135.0 true ; AR 135 to be close to character, but have a little distance. Stop Overlap to not cross with player model
                      (:OnSuccess
                        (Default|Attack (Variables|Default|GetRefEnemy))
                        (Utilities|FlowControl|Sequence ; First move to character to attack using "do once", secondly if doesn't find "Find enemy"
                          (:then_0
                            (goto _label_2 Reset))
                          (:then_1
                            (goto _label))))
                      (:OnFail
                        (Utilities|FlowControl|Delay 1.0)
                        (Utilities|FlowControl|Sequence ; First move to character using "do once", secondly if doesn't find then "Find enemy"
                          (:then_0
                            (goto _label_2 Reset))
                          (:then_1
                            (goto _label)))))))
                (else
                  ;[0.15 0.15 0.15 0.5] If enemy didn't found player from the start, using their location he will start to patrol the area with radius of 1200
                  (Utilities|FlowControl|DoOnce false :!label _label_3
                    (:Completed
                      (AI|AIMoveTo (Variables|Default|GetRefEnemy) (.RandomLocation (AI|Navigation|GetRandomReachablePointinRadius (Transformation|GetActorLocation (Variables|Default|GetRefEnemy)) 1.2e+03 0 0)) 0 135.0 true ; Stop Overlap to not cross with other models
                        (:then
                          (Utilities|FlowControl|Delay 4.0)
                          (goto _label_3 Reset))))))))))))))

(fn ConstructionScript)

(fn FindEnemy
  ;[0.15 0.15 0.15 0.5] First checking if main character is alive, false output when player is dead
  (bind _asbp_ch_player (Utilities|Casting|CastToBP_CH_Player (Game|GetPlayerCharacter 0))
    (:then
      ;[0.15 0.15 0.15 0.5] The logic of detecting a player as an enemy. Two conditions: If distance to main character less than 2000 - player found, if more than 2000 - player alive, but didn't found
      (if (< (Transformation|GetDistanceTo (Variables|Default|GetRefEnemy) (Variables|Default|GetRefPlayer)) 2e+03)
        (return true (Variables|/Game/VGAProject/Characters/Main_Character/Blueprint/BP_CH_Player.BP_CH_Player_C|GetDead _asbp_ch_player))
        (else
          (return false (Variables|/Game/VGAProject/Characters/Main_Character/Blueprint/BP_CH_Player.BP_CH_Player_C|GetDead _asbp_ch_player)))))
    (:CastFailed
      (return false (Variables|/Game/VGAProject/Characters/Main_Character/Blueprint/BP_CH_Player.BP_CH_Player_C|GetDead _asbp_ch_player)))))